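; BP_HS_Pawn_A is a Harvester of Souls pawn driven by a game controller through a SimpleController target.
; On BeginPlay it binds to the controller's axis-moved delegate, and its axis handler stores the device whose DeviceIndex matches the pawn's PlayerID.
; Each Tick it polls that device's axis values, feeding axis 1 to MoveActor and axis 0 to RotateActor.
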(event `self.ReceiveBeginPlay`
  (add `SimpleControllerBPLibrary.onaxisMovedEventDelegate` (`SimpleControllerBPLibrary.getSimpleControllerTarget`) (`|CreateDelegate` :!event `OnAxisValueChanged`))
  (`parent.ReceiveBeginPlay`))

(event `OnAxisValueChanged`
  (params (deviceID :type String) (axisID :type Integer) (axisValue :type "Float (single-precision)") (deviceIndex :type Integer) (device :type "SimpleControllerDevice Structure") (connectionIndex :type Integer))
  (if (== deviceIndex (`self.PlayerID`))
    (set `self.Device` device)))

(event `self.ReceiveTick`
  (params (DeltaSeconds :type "Float (single-precision)"))
  (bind _axisvalues (`SimpleControllerBPLibrary.getAxisValues` (`self.Device`)))
  (`self.MoveActor` (`BlueprintMapLibrary.Map_Find` _axisvalues 1))
  (`self.RotateActor` (`BlueprintMapLibrary.Map_Find` _axisvalues)))

(fn `UserConstructionScript`
  (`parent.UserConstructionScript`))