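; Player pawn for Harvester of Souls, tracking points and sending round-end score and delayed victory messages to the game state.
; Spawn, unspawn and reset use a scale timeline with visibility toggling, which disables mesh collision when visible and enables it when hidden.
; Per-player axis events look up pawns by ID for forward movement, wired only for players one and two.
; All rotation inputs are unconnected.
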(event `self.ReceiveBeginPlay`
  (`self.ToggleVisibility` false)
  (`self.OnSpawn`)
  (set `self.InitialTransform` (`self.GetTransform`)))

(event `/Game/Harvester_of_Souls/Blueprints/Core/BPI_GameMode.PerformVictory`
  (`KismetSystemLibrary.Delay` 2.0)
  (message `/Game/Harvester_of_Souls/Blueprints/Core/BPI_GameMode.GameOver` (`GameplayStatics.GetGameState`)))

(event `/Game/Harvester_of_Souls/Blueprints/Core/BPI_GameMode.RoundEnd`
  (message `/Game/Harvester_of_Souls/Blueprints/Core/BPI_GameMode.ClaculateScore` (`GameplayStatics.GetGameState`) (`self.PlayerID`) (`self.Points`)))

(event `OnSpawn`
  (set `self.bSpawn` true)
  (`self.ToggleVisibility` true)
  (bind (_direction _alpha) (`Timeline|ToggleSpawn` :!via `PlayFromStart` :!label _label)
    (:`Update`
      (`SceneComponent.SetWorldScale3D` (`self.Mesh`) (`KismetMathLibrary.MakeVector` _alpha _alpha _alpha)))
    (:`Finished`
      (if (not (`self.bSpawn`))
        (`self.ToggleVisibility` false)))))

(event `OnUnspawn`
  (set `self.bSpawn` false)
  (goto _label :!via `ReverseFromEnd`))

(event `/Game/Harvester_of_Souls/Blueprints/Core/BPI_GameMode.RoundStart`)

(event `InputAxis|P1_MoveForward`
  (params (AxisValue :type "Float (single-precision)"))
  (`self.MoveActor` (`/Game/Harvester_of_Souls/Blueprints/Core/BFL_SceneHelpers.GetPawnById` 0) AxisValue))

(event `InputAxis|P2_MoveForward`
  (params (AxisValue :type "Float (single-precision)"))
  (`self.MoveActor` (`/Game/Harvester_of_Souls/Blueprints/Core/BFL_SceneHelpers.GetPawnById` 1) AxisValue))

(event `InputAxis|P3_MoveForward`
  (params (AxisValue :type "Float (single-precision)")))

(event `InputAxis|P4_MoveForward`
  (params (AxisValue :type "Float (single-precision)")))

(event `InputAxis|P2_Rotate`
  (params (AxisValue :type "Float (single-precision)")))

(event `InputAxis|P3_Rotate`
  (params (AxisValue :type "Float (single-precision)")))

(event `InputAxis|P4_Rotate`
  (params (AxisValue :type "Float (single-precision)")))

(event `InputAxis|P1_Rotate`
  (params (AxisValue :type "Float (single-precision)")))

(fn `MoveActor`
  (params (Value :type "Float (double-precision)"))
  (if (!= Value 0.0)
    (`self.AddMovementInput` self (`self.GetActorForwardVector` self) (* Value (`self.MovementSpeed`)) false)))

(fn `Reset`
  (`self.K2_SetActorTransform` (`self.InitialTransform`) false true)
  (set `self.Points` 0)
  (`self.OnSpawn`))

(fn `RotateActor`
  (params (Axis :type "Float (double-precision)") (NewParam :type "/Game/Harvester_of_Souls/Blueprints/Core/BP_HS_Pawn Object Reference"))
  (bind (_returnvalue_roll _returnvalue_pitch _returnvalue_yaw) (`KismetMathLibrary.BreakRotator` (`self.K2_GetActorRotation` NewParam)))
  (if (!= Axis 0.0)
    (`SceneComponent.K2_SetWorldRotation` (`Actor.RootComponent` NewParam) (`KismetMathLibrary.MakeRotator` _returnvalue_roll _returnvalue_pitch (+ _returnvalue_yaw (* Axis (`self.MovementSpeed`)))) false false)))

(fn `ToggleVisibility`
  (params (State :type Boolean))
  (bind _mesh (`self.Mesh`))
  (`SceneComponent.SetVisibility` _mesh State false)
  (`PrimitiveComponent.SetCollisionEnabled` _mesh (select `bool` State :`false` "QueryAndPhysics" :`true` "NoCollision" :!type "ECollisionEnabled Enum")))

(fn `UserConstructionScript`)