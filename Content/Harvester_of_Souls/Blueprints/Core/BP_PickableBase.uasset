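; Base pickable for Harvester of Souls that awards points to the player pawn when its "harvester"-tagged component overlaps the sphere, or expires after a set lifetime.
; A Visibility timeline scales the pickup in on spawn and reverses to shrink and destroy it.
; A second timeline loops forward and backward with a flipped step to bob the mesh.
; A Busy flag prevents repeat collection, and the unspawn particle differs for collected versus expired pickups.
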(event `self.ReceiveBeginPlay`
  (`self.OnSpawn`)
  (`KismetSystemLibrary.K2_SetTimerDelegate` (`|CreateDelegate` :!event `OnLifetimeExpired`) (`self.Lifetime`)))

(event `OnSpawn`
  (bind (_direction _alpha) (`Timeline|Visibility` :!via `PlayFromStart` :!label _label)
    (:`Update`
      (`SceneComponent.SetWorldScale3D` (`self.DefaultSceneRoot`) (`KismetMathLibrary.MakeVector` _alpha _alpha _alpha)))
    (:`Finished`
      (switch `ETimelineDirection` _direction
        (:`Forward`
          (`self.OnActivate`))
        (:`Backward`
          (`self.K2_DestroyActor`))))))

(event `OnUnspawn`
  (params (Collected :type Boolean))
  (`self.UnspawnEffect` Collected)
  (goto _label :!via `ReverseFromEnd`))

(event `UnspawnEffect`
  (params (Collected :type Boolean))
  (`ParticleSystemComponent.SetTemplate` (`self.ParticleSystem`) (select `bool` Collected :`false` "/Game/Harvester_of_Souls/Particles/P_ky_impact.P_ky_impact" :`true` "/Game/Harvester_of_Souls/Particles/P_ky_impact_Blue.P_ky_impact_Blue" :!type "ParticleSystem Object Reference"))
  (`ActorComponent.Activate` (`self.ParticleSystem`) false))

(event `OnActivate`
  (set `self.Step` 5.0)
  (bind (_direction _alpha) (`Timeline|Timeline` :!via `PlayFromStart` :!label _label_2)
    (:`Update`
      (`SceneComponent.K2_AddLocalOffset` (`self.SM_Item`) (`KismetMathLibrary.MakeVector` 0.0 0.0 (* _alpha (`self.Step`))) false false))
    (:`Finished`
      (switch `ETimelineDirection` _direction
        (:`Forward`
          (`self.OnReverse`))
        (:`Backward`
          (`self.OnActivate`))))))

(event `OnReverse`
  (set `self.Step` -5.0)
  (goto _label_2 :!via `ReverseFromEnd`))

(event `self.Sphere.OnComponentBeginOverlap`
  (params (OverlappedComponent :type "PrimitiveComponent Object Reference") (OtherActor :type "Actor Object Reference") (OtherComp :type "PrimitiveComponent Object Reference") (OtherBodyIndex :type Integer) (bFromSweep :type Boolean) (SweepResult :type "HitResult Structure (by ref)"))
  (bind (_asbp_hs_pawn _bsuccess) (cast `/Game/Harvester_of_Souls/Blueprints/Core/BP_HS_Pawn` OtherActor :!pure true))
  (if (and _bsuccess (`ActorComponent.ComponentHasTag` OtherComp "harvester"))
    (if (not (`self.bBusy`))
      (set `self.bBusy` true)
      (`/Game/Harvester_of_Souls/Blueprints/Core/BP_HS_Pawn.UpdatePlayerScore` _asbp_hs_pawn (`self.Points`))
      (`self.OnUnspawn` true))))

(event `OnLifetimeExpired`
  (`self.OnUnspawn` false))

(fn `UserConstructionScript`)