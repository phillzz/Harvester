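; Foliage controller for Harvester of Souls that spawns a square grid of BP_HS_FoliageUnit actors offset from its own location, with X and Y swapped.
; GenerateField runs from the construction script and on RoundStart, clearing and refilling its instance array without destroying existing units.
; Reset destroys every foliage unit in the level and regenerates the field, though nothing here calls it.
; BeginPlay and RestartRound are empty.
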(event `self.ReceiveBeginPlay`)

(event `/Game/Harvester_of_Souls/Blueprints/Core/BPI_GameMode.RestartRound`)

(event `/Game/Harvester_of_Souls/Blueprints/Core/BPI_GameMode.RoundStart`
  (`self.Generate Field`))

(fn `Generate Field`
  (bind (_returnvalue_x _returnvalue_y) (`KismetMathLibrary.BreakVector` (`self.K2_GetActorLocation`)))
  (`KismetArrayLibrary.Array_Clear` (`self.FoliageInstances`))
  (for _index (range 22)
    (for _index_2 (range 22)
      (bind _returnvalue (`|SpawnActorFromClass` "/Game/Harvester_of_Souls/Blueprints/Core/BP_HS_FoliageUnit.BP_HS_FoliageUnit_C" (`KismetMathLibrary.MakeTransform` (`KismetMathLibrary.MakeVector` (+ (`KismetMathLibrary.Conv_IntToDouble` (* _index_2 350)) _returnvalue_y) (+ _returnvalue_x (* _index 350)))) "Undefined" "MultiplyWithRoot" null null))
      (`KismetArrayLibrary.Array_Add` (`self.FoliageInstances`) _returnvalue))))

(fn `Reset`
  (bind _outactors (`GameplayStatics.GetAllActorsOfClass` "/Game/Harvester_of_Souls/Blueprints/Core/BP_HS_FoliageUnit.BP_HS_FoliageUnit_C"))
  (for _array_element _outactors
    (`self.K2_DestroyActor` _array_element))
  (`self.Generate Field`))

(fn `UserConstructionScript`
  (`self.Generate Field`))