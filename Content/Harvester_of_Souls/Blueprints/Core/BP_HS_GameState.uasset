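; Game state for Harvester of Souls that runs the round loop, from pre-game countdown through timed play to scoring, restart and game over.
; Countdowns spawned through the HUD drive the phase switch, with round start and end messages broadcast to every pawn.
; Once four player scores arrive, the top value's array index becomes the winner ID.
; That pawn teleports to the winning point to celebrate while the others unspawn.
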(event `/Game/Harvester_of_Souls/Blueprints/Core/BPI_GameMode.InitializeGameLoop`
  ;[0.149 0.4688 0.05625] On Game Start
  (`self.Reset`))

(event `/Game/Harvester_of_Souls/Blueprints/Core/BPI_GameMode.OnCountdownEnd`
  ;[0.6654 0.08866 0.07619] Handle Game Loop
  (`KismetSystemLibrary.Delay` 0.2)
  (switch `/Game/Harvester_of_Souls/Blueprints/Core/E_Countdown` (`self.GamePhaseType`)
    (:`NewEnumerator0`
      (`self.HandleRoundStart`))
    (:`NewEnumerator1`
      (`self.HandleRoundEnd`))))

(event `/Game/Harvester_of_Souls/Blueprints/Core/BPI_GameMode.ClaculateScore`
  (params (PlayerID :type Integer) (Score :type Integer))
  (bind _score (`self.Score`))
  ;[0.6654 0.08866 0.07619] Handle Score calculation
  (`BlueprintMapLibrary.Map_Add` _score PlayerID Score)
  (bind _values (`BlueprintMapLibrary.Map_Values` _score))
  (if (== (`KismetArrayLibrary.Array_Length` _values) 4)
    (bind (_indexofmaxvalue _maxvalue) (`KismetMathLibrary.MaxOfIntArray` _values))
    (set `self.WinnerPlayerID` _indexofmaxvalue)
    (set `self.WinnerScore` _maxvalue)
    (`self.HandleWinningState`)))

(event `/Game/Harvester_of_Souls/Blueprints/Core/BPI_GameMode.RestartRound`
  ;[0.6654 0.08866 0.07619] Handle Round Restart
  (bind _outactors (`GameplayStatics.GetAllActorsOfClass` "/Game/Harvester_of_Souls/Blueprints/Core/BP_HS_Pawn.BP_HS_Pawn_C"))
  (for _array_element _outactors
    (`/Game/Harvester_of_Souls/Blueprints/Core/BP_HS_Pawn.Reset` _array_element))
  (`self.Reset`))

(event `/Game/Harvester_of_Souls/Blueprints/Core/BPI_GameMode.GameOver`
  ;[0.6654 0.08866 0.07619] Handle Game Over
  (bind _outactors (`GameplayStatics.GetAllActorsOfClass` "/Game/Harvester_of_Souls/Blueprints/Core/BP_HS_HUD.BP_HS_HUD_C"))
  (`/Game/Harvester_of_Souls/Blueprints/Core/BP_HS_HUD.evt_GameOver` (`|GetArrayItem` _outactors)))

(fn `GetTimerInitValue`
  (returns (Value :type Integer))
  (return (select `/Game/Harvester_of_Souls/Blueprints/Core/E_Countdown` (`self.GamePhaseType`) :`NewEnumerator0` (`self.PreGameCountdown`) :`NewEnumerator1` (`self.GameCountdown`))))

(fn `HandleRoundEnd`
  (locals (MaxPoints :type Integer) (ID :type Integer) (pawns :type "/Game/Harvester_of_Souls/Blueprints/Core/BP_HS_Pawn Object Reference"))
  (bind _outactors (`GameplayStatics.GetAllActorsOfClass` "/Game/Harvester_of_Souls/Blueprints/Core/BP_HS_Pawn.BP_HS_Pawn_C"))
  (for _array_element _outactors
    (message `/Game/Harvester_of_Souls/Blueprints/Core/BPI_GameMode.RoundEnd` _array_element)))

(fn `HandleRoundStart`
  (set `self.GamePhaseType` "NewEnumerator1")
  (bind _outactors (`GameplayStatics.GetAllActorsOfClass` "/Game/Harvester_of_Souls/Blueprints/Core/BP_HS_Pawn.BP_HS_Pawn_C"))
  (for _array_element _outactors
    (message `/Game/Harvester_of_Souls/Blueprints/Core/BPI_GameMode.RoundStart` _array_element))
  (`self.StartCountdown`))

(fn `HandleWinningState`
  (bind _outactors (`GameplayStatics.GetAllActorsOfClass` "/Game/Harvester_of_Souls/Blueprints/Core/BP_HS_Pawn.BP_HS_Pawn_C"))
  (for _array_element _outactors
    (if (!= (`/Game/Harvester_of_Souls/Blueprints/Core/BP_HS_Pawn.PlayerID` _array_element) (`self.WinnerPlayerID`))
      (`/Game/Harvester_of_Souls/Blueprints/Core/BP_HS_Pawn.OnUnspawn` _array_element)
      (else
        (bind _returnvalue (`GameplayStatics.GetActorOfClass` "/Game/Harvester_of_Souls/Blueprints/Core/BP_WinningPoint.BP_WinningPoint_C"))
        (`self.K2_SetActorTransform` _array_element (`self.GetTransform` _returnvalue) false true)
        (message `/Game/Harvester_of_Souls/Blueprints/Core/BPI_GameMode.PerformVictory` _array_element)))))

(fn `Reset`
  (`|ExecutionSequence`
    (:`then_0`
      (set `self.GamePhaseType` "NewEnumerator0"))
    (:`then_1`
      (`self.StartCountdown`))
    (:`then_2`
      (`BlueprintMapLibrary.Map_Clear` (`self.Score`))
      (set `self.WinnerScore` 0)
      (set `self.WinnerPlayerID` 0))))

(fn `StartCountdown`
  (bind _outactors (`GameplayStatics.GetAllActorsOfClass` "/Game/Harvester_of_Souls/Blueprints/Core/BP_HS_HUD.BP_HS_HUD_C"))
  (`/Game/Harvester_of_Souls/Blueprints/Core/BP_HS_HUD.SpawnCountdown` (`|GetArrayItem` _outactors)))

(fn `UserConstructionScript`)