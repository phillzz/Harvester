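; BP_HS_BorderComponent turns its owning TriggerBox into a border that returns overlapping BP_HS_Pawn actors to their player start.
; On BeginPlay it binds to the box's actor overlap event.
; On overlap it searches all BP_PlayerStart actors for a matching PlayerID and teleports the pawn there without sweep.
; An OnBorderOverlap call on the pawn is present but never runs.
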(event `self.ReceiveBeginPlay`
  (bind _astrigger_box (cast `TriggerBox` (`self.GetOwner`)))
  (add `Actor.OnActorBeginOverlap` _astrigger_box (`|CreateDelegate` :!event `OnBeginOverlap`)))

(event `OnBeginOverlap`
  (params (OverlappedActor :type "Actor Object Reference") (OtherActor :type "Actor Object Reference"))
  (bind _asbp_hs_pawn (cast `/Game/Harvester_of_Souls/Blueprints/Core/BP_HS_Pawn` OtherActor))
  (bind _outactors (`GameplayStatics.GetAllActorsOfClass` "/Game/Harvester_of_Souls/Blueprints/Core/BP_PlayerStart.BP_PlayerStart_C"))
  (for _array_element _outactors
    (if (== (`/Game/Harvester_of_Souls/Blueprints/Core/BP_PlayerStart.PlayerID` _array_element) (`/Game/Harvester_of_Souls/Blueprints/Core/BP_HS_Pawn.PlayerID` _asbp_hs_pawn))
      (`Actor.K2_SetActorLocation` _asbp_hs_pawn (`Actor.K2_GetActorLocation` _array_element) false true))))