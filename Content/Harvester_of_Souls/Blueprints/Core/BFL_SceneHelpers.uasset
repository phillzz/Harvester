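; Blueprint function library of scene lookup helpers for Harvester of Souls that finds player objects by ID.
; One function searches all BP_HS_PlayerController actors and another all BP_HS_Pawn actors, each returning the first whose PlayerID matches.
; Both do a linear GetAllActorsOfClass scan on every call rather than using a cached registry.
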(fn `GetPawnById`
  (params (ID :type Integer))
  (returns (Pawn :type "/Game/Harvester_of_Souls/Blueprints/Core/BP_HS_Pawn Object Reference"))
  (bind _outactors (`GameplayStatics.GetAllActorsOfClass` (`local.__WorldContext`) "/Game/Harvester_of_Souls/Blueprints/Core/BP_HS_Pawn.BP_HS_Pawn_C"))
  (for _array_element _outactors
    (if (== (`/Game/Harvester_of_Souls/Blueprints/Core/BP_HS_Pawn.PlayerID` _array_element) ID)
      (return _array_element))))

(fn `GetPlayerControllerById`
  (params (`ID(0-3)` :type Integer))
  (returns (PlayerController :type "/Game/Harvester_of_Souls/Blueprints/Core/BP_HS_PlayerController Object Reference"))
  (bind _outactors (`GameplayStatics.GetAllActorsOfClass` (`local.__WorldContext`) "/Game/Harvester_of_Souls/Blueprints/Core/BP_HS_PlayerController.BP_HS_PlayerController_C"))
  (for _array_element _outactors
    (if (== (`/Game/Harvester_of_Souls/Blueprints/Core/BP_HS_PlayerController.PlayerID` _array_element) `ID(0-3)`)
      (return _array_element))))