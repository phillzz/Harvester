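; BP_HS_FoliageUnit is a harvestable crop patch, built in the construction script as a 6x6 grid of randomly yawed hierarchical instanced meshes.
; A Grow timeline scales the mesh component up on spawn.
; The first overlap by a moving BP_HS_Pawn's "harvester"-tagged component reverses Grow to shrink it.
; SlowGrow then regrows the patch, lerping a dynamic material's Tint from green to golden, with no further harvesting.
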(event `self.ReceiveBeginPlay`
  (`self.OnSpawn`))

(event `OnSpawn`
  (bind _hierarchicalinstancedstaticmesh (`self.HierarchicalInstancedStaticMesh`))
  (bind (_direction _alpha) (`Timeline|Grow` :!via `PlayFromStart` :!label _label)
    (:`Update`
      (`SceneComponent.SetWorldScale3D` (`self.HierarchicalInstancedStaticMesh`) (`KismetMathLibrary.MakeVector` _alpha _alpha _alpha)))
    (:`Finished`
      (switch `ETimelineDirection` _direction
        (:`Backward`
          (bind _returnvalue (`PrimitiveComponent.CreateDynamicMaterialInstance` _hierarchicalinstancedstaticmesh 1 (`PrimitiveComponent.GetMaterial` _hierarchicalinstancedstaticmesh 1) "None"))
          (bind _output_get (set `self.DMI` _returnvalue))
          (`MaterialInstanceDynamic.SetVectorParameterValue` _returnvalue "Tint" (struct :`G` 1.0 :`B` 0.059439 :`A` 1.0))
          (`MaterialInstanceDynamic.SetVectorParameterValue` _output_get "Tint" (struct :`G` 1.0 :`B` 0.059439 :`A` 1.0))
          (bind (_direction_2 _alpha_2) (`Timeline|SlowGrow` :!via `PlayFromStart`)
            (:`Update`
              (`SceneComponent.SetWorldScale3D` (`self.HierarchicalInstancedStaticMesh`) (`KismetMathLibrary.MakeVector` _alpha_2 _alpha_2 _alpha_2))
              (`MaterialInstanceDynamic.SetVectorParameterValue` (`self.DMI`) "Tint" (`KismetMathLibrary.LinearColorLerp` (struct :`G` 1.0 :`B` 0.059439 :`A` 1.0) (struct :`R` 1.7 :`G` 1.179583 :`B` 0.565168 :`A` 1.0) _alpha_2)))))))))

(event `OnUnspawn`
  (goto _label :!via `ReverseFromEnd`))

(event `self.Box.OnComponentBeginOverlap`
  (params (OverlappedComponent :type "PrimitiveComponent Object Reference") (OtherActor :type "Actor Object Reference") (OtherComp :type "PrimitiveComponent Object Reference") (OtherBodyIndex :type Integer) (bFromSweep :type Boolean) (SweepResult :type "HitResult Structure (by ref)"))
  (bind _asbp_hs_pawn (cast `/Game/Harvester_of_Souls/Blueprints/Core/BP_HS_Pawn` OtherActor))
  (if (`/Game/Harvester_of_Souls/Blueprints/Core/BP_HS_Pawn.bMovement` _asbp_hs_pawn)
    (if (and (not (`self.bUsed`)) (`ActorComponent.ComponentHasTag` OtherComp "harvester"))
      (set `self.bUsed` true)
      (`self.OnUnspawn`))))

(fn `UserConstructionScript`
  (bind (_returnvalue_roll _returnvalue_pitch _returnvalue_yaw) (`KismetMathLibrary.BreakRotator` (`KismetMathLibrary.RandomRotator` false)))
  (for _index (range 6)
    (for _index_2 (range 6)
      (`InstancedStaticMeshComponent.AddInstance` (`self.HierarchicalInstancedStaticMesh`) (`KismetMathLibrary.MakeTransform` (`KismetMathLibrary.MakeVector` (`KismetMathLibrary.Conv_IntToDouble` (* _index_2 70)) (`KismetMathLibrary.Conv_IntToDouble` (* _index 70))) (`KismetMathLibrary.MakeRotator` -10.0 10.0 _returnvalue_yaw)) false))))