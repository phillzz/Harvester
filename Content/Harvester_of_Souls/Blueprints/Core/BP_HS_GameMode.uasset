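; Game mode for Harvester of Souls that sets up local multiplayer for up to four players on BeginPlay.
; It removes existing players, then creates a local player and controller ID for each BP_PlayerStart index with a matching PlayerID.
; Each player possesses an index-selected pawn class (A–D) and views through a shared level CameraActor.
; Finally, it messages the game state to initialize the game loop.
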(event `self.ReceiveBeginPlay`
  (`self.SpawnPlayers`))

(fn `GetPlayerStartPoints`
  (returns (PlayerStartPoints :type "Array of /Game/Harvester_of_Souls/Blueprints/Core/BP_PlayerStart Object Reference"))
  (bind _outactors (`GameplayStatics.GetAllActorsOfClass` "/Game/Harvester_of_Souls/Blueprints/Core/BP_PlayerStart.BP_PlayerStart_C"))
  (bind _output_get (set `self.StartPoints` _outactors))
  (return _output_get))

(fn `Reset`
  (for _index (range 4)
    (bind _playercontroller (`/Game/Harvester_of_Souls/Blueprints/Core/BFL_SceneHelpers.GetPlayerControllerById` _index))
    (`/Engine/EditorBlueprintResources/StandardMacros.IsValid` _playercontroller
      (:`Is Valid`
        (`GameplayStatics.RemovePlayer` _playercontroller true)))))

(fn `SpawnPlayers`
  (locals (CurrentIndex :type Integer))
  (bind _playerstartpoints (`self.GetPlayerStartPoints`))
  (bind _currentindex (`local.CurrentIndex`))
  (bind _returnvalue (`GameplayStatics.GetPlayerController` (`local.CurrentIndex`)))
  (`self.Reset`)
  (bind _returnvalue_2 (`GameplayStatics.GetActorOfClass` "/Script/Engine.CameraActor"))
  (for (_ _array_index) _playerstartpoints
    (bind _output_get (set `local.CurrentIndex` _array_index))
    (for _array_element _playerstartpoints
      (if (== (`/Game/Harvester_of_Souls/Blueprints/Core/BP_PlayerStart.PlayerID` _array_element) _output_get)
        (bind _returnvalue_3 (`GameplayStatics.CreatePlayerFromPlatformUser` (`InputDeviceLibrary.PlatformUserId_None`)))
        (`GameplayStatics.SetPlayerControllerID` _returnvalue_3 _currentindex)
        (bind _asbp_hs_pawn (castclass `/Game/Harvester_of_Souls/Blueprints/Core/BP_HS_Pawn` (select `int` (`local.CurrentIndex`) :`0` "/Game/Harvester_of_Souls/Blueprints/BP_HS_Pawn_A.BP_HS_Pawn_A_C" :`1` "/Game/Harvester_of_Souls/Blueprints/BP_HS_Pawn_B.BP_HS_Pawn_B_C" :`2` "/Game/Harvester_of_Souls/Blueprints/BP_HS_Pawn_C.BP_HS_Pawn_C_C" :`3` "/Game/Harvester_of_Souls/Blueprints/BP_HS_Pawn_D.BP_HS_Pawn_D_C" :!type "Actor Class Reference")))
        (bind _returnvalue_4 (`|SpawnActorFromClass` _asbp_hs_pawn (`self.GetTransform` (`|GetArrayItem` (`self.StartPoints`) _currentindex)) "Undefined" "MultiplyWithRoot" null _currentindex null))
        (`Controller.Possess` _returnvalue _returnvalue_4)
        (`PlayerController.SetViewTargetWithBlend` _returnvalue _returnvalue_2 0.0 "VTBlend_Linear" 0.0 false))))
  (message `/Game/Harvester_of_Souls/Blueprints/Core/BPI_GameMode.InitializeGameLoop` (`GameplayStatics.GetGameState`)))

(fn `UserConstructionScript`)