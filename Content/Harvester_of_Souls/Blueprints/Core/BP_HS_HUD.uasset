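; HUD Blueprint for Harvester of Souls that manages the on-screen WBP_GameMenu message widget.
; SpawnUI creates the widget once, adds it to the viewport and runs its Setup, which StartCountdown calls again.
; On game over it displays "Game Over!", then after the game state's message delay calls RestartRoundMessage on the game state.
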(event `evt_GameOver`
  (`/Game/Harvester_of_Souls/UI/WBP_GameMenu.SetMessage` (`self.Message`) "Game Over!")
  (`KismetSystemLibrary.K2_SetTimerDelegate` (delegate `OnGameOverEnd`) (`/Game/Harvester_of_Souls/Blueprints/Core/BP_HS_GameState.GetMessageDelay` (`/Game/Harvester_of_Souls/Blueprints/Core/BFL_Helpers.HS_GetGameState`))))

(event `OnGameOverEnd`
  (message `/Game/Harvester_of_Souls/Blueprints/Core/BPI_GameMode.RestartRound` (`GameplayStatics.GetGameState`)))

(fn `SpawnUI`
  (`/Engine/EditorBlueprintResources/StandardMacros.IsValid` (`self.Message`)
    (:`Is Valid`
      _)
    (:`Is Not Valid`
      (bind _returnvalue (`|CreateWidget` "/Game/Harvester_of_Souls/UI/WBP_GameMenu.WBP_GameMenu_C" (`GameplayStatics.GetPlayerController` 0)))
      (bind _output_get (set `self.Message` _returnvalue))))
  (if (not (`Widget.IsInViewport` _output_get))
    (`UserWidget.AddToViewport` _output_get 0))
  (`/Game/Harvester_of_Souls/UI/WBP_GameMenu.Setup` _output_get))

(fn `StartCountdown`
  (`/Game/Harvester_of_Souls/UI/WBP_GameMenu.Setup` (`self.Message`)))

(fn `UserConstructionScript`)