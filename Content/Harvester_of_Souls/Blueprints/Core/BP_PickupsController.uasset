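; Pickup controller actor that keeps the level stocked with randomly placed pickups in Harvester of Souls.
; On BeginPlay it starts a looping one-second timer that calls SpawnPickable.
; Each call counts existing actors of a class and, below four, spawns one of four randomly selected classes.
; Spawns land at random X/Y within a box around the world origin at fixed height, adjusted for collision or skipped if still blocked.
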(event `self.ReceiveBeginPlay`
  (bind _returnvalue (`KismetSystemLibrary.K2_SetTimer` null "SpawnPickable" 1.0 true))
  (set `self.Timer` _returnvalue))

(fn `SpawnPickable`
  (bind (_returnvalue_x _returnvalue_y) (`KismetMathLibrary.BreakVector` (`KismetMathLibrary.RandomPointInBoundingBox` (0.0 0.0 50.0) (2500.0 2500.0 50.0))))
  (bind _outactors (`GameplayStatics.GetAllActorsOfClass` null))
  (if (< (`KismetArrayLibrary.Array_Length` _outactors) 4)
    (`|SpawnActorFromClass` (select `int` (`KismetMathLibrary.RandomIntegerInRange` 0 3) :`0` null :`1` null :`2` null :`3` null :!type "Actor Class Reference") (`KismetMathLibrary.MakeTransform` (`KismetMathLibrary.MakeVector` _returnvalue_x _returnvalue_y 125.0)) "AdjustIfPossibleButDontSpawnIfColliding" "MultiplyWithRoot" null null)))

(fn `UserConstructionScript`)