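; BP_HS_Pawn_B is a Harvester of Souls pawn driven by axis input from an external Simple Controller device.
; On BeginPlay it binds a handler to the controller target's axis-moved delegate, then runs the parent BeginPlay.
; The handler accepts only input whose connection index matches the pawn's PlayerID, routing the first axis to MoveActor and the second to RotateActor.
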(event `self.ReceiveBeginPlay`
  (add `SimpleControllerBPLibrary.onaxisMovedEventDelegate` (`SimpleControllerBPLibrary.getSimpleControllerTarget`) (`|CreateDelegate` :!event `OnAxisValueChanged`))
  (`parent.ReceiveBeginPlay`))

(event `OnAxisValueChanged`
  (params (deviceID :type String) (axisID :type Integer) (axisValue :type "Float (single-precision)") (deviceIndex :type Integer) (device :type "SimpleControllerDevice Structure") (connectionIndex :type Integer))
  (if (== connectionIndex (`self.PlayerID`))
    (switch `int` axisID
      (:`0`
        (`self.MoveActor` axisValue))
      (:`1`
        (`self.RotateActor` axisValue)))))

(fn `UserConstructionScript`
  (`parent.UserConstructionScript`))